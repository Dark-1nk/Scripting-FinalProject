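; BP_HungerComponent is an actor component that tracks hunger and thirst as survival meters for the top-down character.
; Both meters start full on BeginPlay and drain every Tick at their own rates, clamped between zero and their maximums.
; When either reaches zero, it casts the owner to BP_TopDownChar and calls Death on every tick it stays empty.
; Eat and Drink functions refill the respective meter by a given amount, capped at the maximum.
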(event `self.ReceiveBeginPlay`
  (set `self.HungerCurrent` (`self.HungerMax`))
  (set `self.ThirstCurrent` (`self.ThirstMax`)))

(event `self.ReceiveTick`
  (params (DeltaSeconds :type "Float (single-precision)"))
  (set `self.HungerCurrent` (`KismetMathLibrary.FClamp` (- (`self.HungerCurrent`) (* DeltaSeconds (`self.HungerDrain`))) 0.0 (`self.HungerMax`)))
  (set `self.ThirstCurrent` (`KismetMathLibrary.FClamp` (- (`self.ThirstCurrent`) (* DeltaSeconds (`self.ThirstDrain`))) 0.0 (`self.ThirstMax`)))
  (if (or (<= (`self.HungerCurrent`) 0.0) (<= (`self.ThirstCurrent`) 0.0))
    (bind _asbp_top_down_char (cast `/Game/Blueprints/Characters/Players/BP_TopDownChar` (`self.GetOwner`)))
    (`/Game/Blueprints/Characters/Players/BP_TopDownChar.Death` _asbp_top_down_char)))

(fn `Drink`
  (params (DrinkAmount :type "Float (double-precision)"))
  (set `self.ThirstCurrent` (`KismetMathLibrary.FClamp` (+ DrinkAmount (`self.ThirstCurrent`)) 0.0 (`self.ThirstMax`))))

(fn `Eat`
  (params (NutritionalValue :type "Float (double-precision)"))
  (set `self.HungerCurrent` (`KismetMathLibrary.FClamp` (+ NutritionalValue (`self.HungerCurrent`)) 0.0 (`self.HungerMax`))))