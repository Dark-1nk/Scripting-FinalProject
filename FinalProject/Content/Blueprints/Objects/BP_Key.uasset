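; BP_Key is a key pickup that sets HasKey on the interacting player character and then destroys itself.
; Its InteractRadius overlap registers the key as the character's CurrentInteractable, and end overlap clears it only if it is still this key.
; Interact casts to BP_TopDownHorrorChar, while the overlap events cast to BP_TopDownChar.
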(event `self.ReceiveTick`
  (params (DeltaSeconds :type "Float (single-precision)")))

(event `self.Interact`
  (params (Interactor :type "/Game/Blueprints/Characters/Players/BP_TopDownChar Object Reference"))
  (bind _asbp_top_down_horror_char (cast `/Game/Blueprints/Characters/Players/BP_TopDownHorrorChar` Interactor))
  (set `/Game/Blueprints/Characters/Players/BP_TopDownHorrorChar.hasKey` true _asbp_top_down_horror_char)
  (`self.K2_DestroyActor`))

(event `self.InteractRadius.OnComponentBeginOverlap`
  (params (OverlappedComponent :type "PrimitiveComponent Object Reference") (OtherActor :type "Actor Object Reference") (OtherComp :type "PrimitiveComponent Object Reference") (OtherBodyIndex :type Integer) (bFromSweep :type Boolean) (SweepResult :type "HitResult Structure (by ref)"))
  (bind _asbp_top_down_char (cast `/Game/Blueprints/Characters/Players/BP_TopDownChar` OtherActor))
  (set `/Game/Blueprints/Characters/Players/BP_TopDownChar.CurrentInteractable` self _asbp_top_down_char))

(event `self.InteractRadius.OnComponentEndOverlap`
  (params (OverlappedComponent :type "PrimitiveComponent Object Reference") (OtherActor :type "Actor Object Reference") (OtherComp :type "PrimitiveComponent Object Reference") (OtherBodyIndex :type Integer))
  (bind _asbp_top_down_char (cast `/Game/Blueprints/Characters/Players/BP_TopDownChar` OtherActor))
  (if (== (`/Game/Blueprints/Characters/Players/BP_TopDownChar.CurrentInteractable` _asbp_top_down_char) self)
    (set `/Game/Blueprints/Characters/Players/BP_TopDownChar.CurrentInteractable` null _asbp_top_down_char)))

(fn `UserConstructionScript`)