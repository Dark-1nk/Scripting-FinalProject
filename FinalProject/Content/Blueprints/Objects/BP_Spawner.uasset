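; Spawner actor that keeps dropping food and drink items at random spots inside its spawn volume for as long as play runs.
; On BeginPlay it starts a self-repeating loop that waits a random few seconds, then spawns either a drink or food actor with equal chance at reduced scale.
; Each spawn location is a random point within the SpawnVolume box component's extent.
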(event `self.ReceiveBeginPlay`
  (`self.StartSpawnLoop`))

(event `StartSpawnLoop`
  (`KismetSystemLibrary.RetriggerableDelay` (`KismetMathLibrary.RandomFloatInRange` 2.0 7.0))
  (`self.TriggerSpawn`))

(event `TriggerSpawn`
  (`|SpawnActorFromClass` (select `bool` (`KismetMathLibrary.RandomBool`) :`false` (`self.FoodActor`) :`true` (`self.DrinkActor`)) (`KismetMathLibrary.MakeTransform` (`self.GetRandomBoxLocation`) (struct) (0.2 0.2 0.2)) "Undefined" "MultiplyWithRoot" null null)
  (`self.StartSpawnLoop`))

(fn `GetRandomBoxLocation`
  (returns (Location :type "Vector Structure"))
  (bind _spawnvolume (`self.SpawnVolume`))
  (return (`KismetMathLibrary.RandomPointInBoundingBox` (`SceneComponent.K2_GetComponentLocation` _spawnvolume) (`BoxComponent.BoxExtent` _spawnvolume))))

(fn `UserConstructionScript`)