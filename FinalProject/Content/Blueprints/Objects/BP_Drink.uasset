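; BP_Drink is a short-lived drink pickup that the player can consume and that destroys itself fifteen seconds after spawning.
; An overlap radius registers it as the top-down hunger character's current interactable and clears that on exit if still set.
; On Interact, it passes its nutritional value to the interactor's hunger component, plays a gulp sound and effect, then destroys itself.
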(event `self.ReceiveBeginPlay`
  (`KismetSystemLibrary.Delay` 15.0)
  (`self.K2_DestroyActor`))

(event `/Game/Blueprints/Core/BPI_Interactable.Interact`
  (params (Interactor :type "/Game/Blueprints/Characters/Players/BP_TopDownChar Object Reference"))
  (bind _returnvalue (`self.GetComponentByClass` Interactor "/Game/Blueprints/Components/BP_HungerComponent.BP_HungerComponent_C"))
  (`/Engine/EditorBlueprintResources/StandardMacros.IsValid` _returnvalue
    (:`Is Valid`
      (`/Game/Blueprints/Components/BP_HungerComponent.Drink` _returnvalue (`self.NutritionalValue`))
      (`GameplayStatics.PlaySound2D` "/Game/Audio/SC_Gulp.SC_Gulp" 1.0 1.0 0.0 null null)
      (`NiagaraFunctionLibrary.SpawnSystemAtLocation` "/Game/Effects/FX_Drink.FX_Drink" (`SceneComponent.K2_GetComponentLocation` (`self.Bottle`)))
      (`self.K2_DestroyActor`))))

(event `self.InteractRadius.OnComponentBeginOverlap`
  (params (OverlappedComponent :type "PrimitiveComponent Object Reference") (OtherActor :type "Actor Object Reference") (OtherComp :type "PrimitiveComponent Object Reference") (OtherBodyIndex :type Integer) (bFromSweep :type Boolean) (SweepResult :type "HitResult Structure (by ref)"))
  (bind _asbp_top_down_hunger_char (cast `/Game/Blueprints/Characters/Players/BP_TopDownHungerChar` OtherActor))
  (set `/Game/Blueprints/Characters/Players/BP_TopDownChar.CurrentInteractable` self _asbp_top_down_hunger_char))

(event `self.InteractRadius.OnComponentEndOverlap`
  (params (OverlappedComponent :type "PrimitiveComponent Object Reference") (OtherActor :type "Actor Object Reference") (OtherComp :type "PrimitiveComponent Object Reference") (OtherBodyIndex :type Integer))
  (bind _asbp_top_down_hunger_char (cast `/Game/Blueprints/Characters/Players/BP_TopDownHungerChar` OtherActor))
  (if (== (`/Game/Blueprints/Characters/Players/BP_TopDownChar.CurrentInteractable` _asbp_top_down_hunger_char) self)
    (set `/Game/Blueprints/Characters/Players/BP_TopDownChar.CurrentInteractable` null _asbp_top_down_hunger_char)))

(fn `UserConstructionScript`)