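; BP_CutscenePlayer is an interactable object that plays the LS_EndScene level sequence.
; Its InteractZone registers it as the CurrentInteractable of an overlapping BP_TopDownChar and clears that reference on exit if it still matches.
; Interact waits briefly, starts the sequence, then immediately sets the player's view target to the PC_PlayerController's CurrentCamera without waiting for playback to finish.
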(event `self.Interact`
  (params (Interactor :type "/Game/Blueprints/Characters/Players/BP_TopDownChar Object Reference"))
  (bind _returnvalue (`GameplayStatics.GetPlayerController` 0))
  (`KismetSystemLibrary.Delay` 0.5)
  (bind (_outactor _returnvalue_2) (`LevelSequencePlayer.CreateLevelSequencePlayer` "/Game/Cutscenes/LS_EndScene.LS_EndScene"))
  (`MovieSceneSequencePlayer.Play` _returnvalue_2)
  (bind _aspc_player_controller (cast `/Game/Blueprints/Core/PC_PlayerController` _returnvalue))
  (`PlayerController.SetViewTargetWithBlend` _returnvalue (`/Game/Blueprints/Core/PC_PlayerController.CurrentCamera` _aspc_player_controller) 0.0 "VTBlend_Linear" 0.0 false))

(event `self.InteractZone.OnComponentBeginOverlap`
  (params (OverlappedComponent :type "PrimitiveComponent Object Reference") (OtherActor :type "Actor Object Reference") (OtherComp :type "PrimitiveComponent Object Reference") (OtherBodyIndex :type Integer) (bFromSweep :type Boolean) (SweepResult :type "HitResult Structure (by ref)"))
  (bind _asbp_top_down_char (cast `/Game/Blueprints/Characters/Players/BP_TopDownChar` OtherActor))
  (set `/Game/Blueprints/Characters/Players/BP_TopDownChar.CurrentInteractable` self _asbp_top_down_char))

(event `self.InteractZone.OnComponentEndOverlap`
  (params (OverlappedComponent :type "PrimitiveComponent Object Reference") (OtherActor :type "Actor Object Reference") (OtherComp :type "PrimitiveComponent Object Reference") (OtherBodyIndex :type Integer))
  (bind _asbp_top_down_char (cast `/Game/Blueprints/Characters/Players/BP_TopDownChar` OtherActor))
  (if (== (`/Game/Blueprints/Characters/Players/BP_TopDownChar.CurrentInteractable` _asbp_top_down_char) self)
    (set `/Game/Blueprints/Characters/Players/BP_TopDownChar.CurrentInteractable` null _asbp_top_down_char)))

(fn `UserConstructionScript`)