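; Battle manager actor that runs turn-based fights between the player and a list of enemies.
; It links itself to the battle UI on the overworld HUD, and StartBattle sets enemy types, flags the battle active and shows that UI.
; Player actions cover attacking the selected enemy, using items and defending, which halves the next incoming hit.
; NextTurn steps an index through the enemies, with -1 marking the player's turn, and notifies the UI.
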(event `self.ReceiveBeginPlay`
  ; Get the Battle UI from the HUD class
  (bind _returnvalue (`GameplayStatics.GetActorOfClass` (`GameModeBase.HUDClass` (`GameplayStatics.GetGameMode`))))
  (bind _asbp_overworld_hud (cast `/Game/Blueprints/Core/BP_OverworldHUD` _returnvalue))
  (bind _output_get (set `self.BattleUI` (`/Game/Blueprints/Core/BP_OverworldHUD.BattleUI` _asbp_overworld_hud)))
  (set `/Game/Blueprints/UI/WBP_BattleUI.BattleManager` self _output_get)
  ; -1 will be the player's turn
  (set `self.TurnIndex` -1))

(event `StartBattle`
  (params (Enemies :type "Array of /Game/DataStructures/E_EnemyTypes Enum"))
  ; Start the battle by getting the list of enemies that the player will fight
  (for (_array_element _array_index) (`self.Enemies`)
    (`/Game/Blueprints/Characters/Enemies/BP_TurnBasedEnemy.SetMyEnemyType` _array_element (`|GetArrayItem` Enemies _array_index)))
  (set `/Game/Blueprints/Characters/Players/BP_TopDownChar.InBattle` true (`self.Player`))
  (set `self.IsBattleActive` true)
  (`Widget.SetVisibility` (`self.BattleUI`) "Visible"))

(event `AttackPlayer`
  (params (Damage :type "Float (double-precision)"))
  ; Deal damage to the player, less if the player chose defend in their last turn
  (`/Game/Blueprints/Characters/Players/BP_TopDownChar.TakeDamage` (`self.Player`) (select `bool` (`self.PlayerDefending`) :`false` Damage :`true` (/ Damage 2.0)))
  (set `self.PlayerDefending` false)
  (`self.NextTurn`))

(event `AttackEnemy`
  (`/Game/Blueprints/Characters/Enemies/BP_TurnBasedEnemy.TakeDamage` (`|GetArrayItem` (`self.Enemies`) (`self.SelectedEnemy`)) (`/Game/Blueprints/Characters/Players/BP_TopDownChar.Damage` (`self.Player`))))

(event `PlayerDefend`
  (set `self.PlayerDefending` true)
  (`self.NextTurn`))

(event `PlayerUseItem`
  (params (item :type "/Game/DataStructures/E_ItemTypes Enum" :default "NewEnumerator0"))
  (`/Game/Blueprints/Characters/Players/BP_TopDownChar.UseItem` (`self.Player`) item)
  (`self.NextTurn`))

(event `NextTurn`
  (bind _battleui (`self.BattleUI`))
  ; Increment the Turn Index. If the index exceeds the amount of enemies, it's the Player's turn. Otherwise, do the next enemy's turn
  (bind _result (`/Engine/EditorBlueprintResources/StandardMacros.IncrementInt` (`self.TurnIndex`))
    (:`  `
      (if (>= _result (`KismetArrayLibrary.Array_Length` (`self.Enemies`)))
        (set `self.TurnIndex` -1)
        (`/Game/Blueprints/UI/WBP_BattleUI.OnPlayerTurn` _battleui)
        (else
          (`/Game/Blueprints/UI/WBP_BattleUI.OnEnemyTurn` _battleui)
          (`/Game/Blueprints/Characters/Enemies/BP_TurnBasedEnemy.OnMyTurn` (`|GetArrayItem` (`self.Enemies`) (`self.TurnIndex`))))))))

(fn `UserConstructionScript`)