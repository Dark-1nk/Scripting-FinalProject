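; BP_RoomTrigger is a room volume that switches the view to its assigned camera when the top-down character enters.
; After a short delay, it confirms the character still overlaps and that the capsule triggered the overlap, then calls ActivateRoom.
; ActivateRoom swaps the player controller's CurrentCamera, updates both cameras' active flags and blends the view target.
; A camera flagged as default activates its room on BeginPlay.
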(event `self.ReceiveBeginPlay`
  (if (`/Game/Blueprints/Visuals/BP_CameraFollow.isDefault` (`self.Camera`))
    (`self.activateRoom`)))

(event `self.ReceiveActorBeginOverlap`
  (params (OtherActor :type "Actor Object Reference")))

(event `self.TriggerBox.OnComponentBeginOverlap`
  (params (OverlappedComponent :type "PrimitiveComponent Object Reference") (OtherActor :type "Actor Object Reference") (OtherComp :type "PrimitiveComponent Object Reference") (OtherBodyIndex :type Integer) (bFromSweep :type Boolean) (SweepResult :type "HitResult Structure (by ref)"))
  (`KismetSystemLibrary.Delay` 0.2)
  (bind _asbp_top_down_char (cast `/Game/Blueprints/Characters/Players/BP_TopDownChar` OtherActor))
  (if (`KismetArrayLibrary.Array_Contains` (`self.GetOverlappingActors` "/Game/Blueprints/Characters/Players/BP_TopDownChar.BP_TopDownChar_C") _asbp_top_down_char)
    (if (== (`Character.CapsuleComponent` _asbp_top_down_char) OtherComp)
      (`self.activateRoom`))))

(fn `activateRoom`
  (bind _aspc_player_controller (cast `/Game/Blueprints/Core/PC_PlayerController` (`GameplayStatics.GetPlayerController` 0)))
  (bind _currentcamera (`/Game/Blueprints/Core/PC_PlayerController.CurrentCamera` _aspc_player_controller))
  (`/Engine/EditorBlueprintResources/StandardMacros.IsValid` _currentcamera
    (:`Is Valid`
      (if (not (== _currentcamera (`self.Camera`)))
        (set `/Game/Blueprints/Visuals/BP_CameraFollow.isActive` false _currentcamera)
        (bind _output_get (set `/Game/Blueprints/Core/PC_PlayerController.CurrentCamera` (`self.Camera`) _aspc_player_controller :!label _label))
        (set `/Game/Blueprints/Visuals/BP_CameraFollow.isActive` true _output_get)
        (`PlayerController.SetViewTargetWithBlend` (`GameplayStatics.GetPlayerController` 0) _output_get 0.5 "VTBlend_Linear" 0.0 false)))
    (:`Is Not Valid`
      (goto _label))))

(fn `UserConstructionScript`)