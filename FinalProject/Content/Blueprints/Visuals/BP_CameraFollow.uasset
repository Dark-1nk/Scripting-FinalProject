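; Camera-follow actor that smoothly trails player pawn 0 with per-axis offsets while active.
; On BeginPlay it derives padded min/max limits on each axis from a referenced BoundingBox's trigger box.
; Each Tick picks one of four view functions by the UseBounds and LockY flags, optionally clamping to those limits or pinning Y to a fixed value.
; All variants move the actor with VInterpTo at FollowSpeed.
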(event `self.ReceiveBeginPlay`
  (bind _triggerbox (`/Game/Blueprints/Visuals/BP_RoomTrigger.TriggerBox` (`self.BoundingBox`)))
  (bind (_returnvalue_x _returnvalue_y _returnvalue_z) (`KismetMathLibrary.BreakVector` (`BoxComponent.GetScaledBoxExtent` _triggerbox)))
  (bind (_returnvalue_x_2 _returnvalue_y_2 _returnvalue_z_2) (`KismetMathLibrary.BreakVector` (`SceneComponent.K2_GetComponentLocation` _triggerbox)))
  (`self.Calculate Bounds` _returnvalue_x_2 _returnvalue_y_2 _returnvalue_z_2 _returnvalue_x _returnvalue_y _returnvalue_z))

(event `self.ReceiveTick`
  (params (DeltaSeconds :type "Float (single-precision)"))
  (bind _locky (`self.LockY`))
  (if (`self.isActive`)
    (if (`self.UseBounds`)
      (if _locky
        (`self.ViewBound` DeltaSeconds)
        (else
          (`self.ViewBoundUnlockedY` DeltaSeconds)))
      (elif _locky
        (`self.ViewUnbound` DeltaSeconds)
        (else
          (`self.ViewUnboundUnlockedY` DeltaSeconds))))))

(fn `Calculate Bounds`
  (params (BoxCenterX :type "Float (double-precision)") (BoxCenterY :type "Float (double-precision)") (BoxCenterZ :type "Float (double-precision)") (BoxExtentX :type "Float (double-precision)") (BoxExtentY :type "Float (double-precision)") (BoxExtentZ :type "Float (double-precision)"))
  (bind _paddingx (`self.PaddingX`))
  (bind _paddingy (`self.PaddingY`))
  (bind _paddingz (`self.PaddingZ`))
  (set `self.MinX` (+ (- BoxCenterX BoxExtentX) _paddingx))
  (set `self.MaxX` (- (+ BoxCenterX BoxExtentX) _paddingx))
  (set `self.MaxY` (- (+ BoxCenterY BoxExtentY) _paddingy))
  (set `self.MinY` (+ (- BoxCenterY BoxExtentY) _paddingy))
  (set `self.MaxZ` (- (+ BoxCenterZ BoxExtentZ) _paddingz))
  (set `self.MinZ` (+ (- BoxCenterZ BoxExtentZ) _paddingz)))

(fn `UserConstructionScript`)

(fn `ViewBound`
  (params (DeltaTime :type "Float (single-precision)"))
  (`self.K2_SetActorLocation` (`KismetMathLibrary.VInterpTo` (`self.K2_GetActorLocation`) (`KismetMathLibrary.MakeVector` (`KismetMathLibrary.FClamp` (+ (`self.OffsetX`) (.x (`self.K2_GetActorLocation` (`GameplayStatics.GetPlayerPawn` 0)))) (`self.MinX`) (`self.MaxX`)) (`self.LockedY`) (`KismetMathLibrary.FClamp` (+ (.z (`self.K2_GetActorLocation` (`GameplayStatics.GetPlayerPawn` 0))) (`self.OffsetZ`)) (`self.MinZ`) (`self.MaxZ`))) DeltaTime (`self.FollowSpeed`))))

(fn `ViewBoundUnlockedY`
  (params (DeltaTime :type "Float (single-precision)"))
  (`self.K2_SetActorLocation` (`KismetMathLibrary.VInterpTo` (`self.K2_GetActorLocation`) (`KismetMathLibrary.MakeVector` (`KismetMathLibrary.FClamp` (+ (`self.OffsetX`) (.x (`self.K2_GetActorLocation` (`GameplayStatics.GetPlayerPawn` 0)))) (`self.MinX`) (`self.MaxX`)) (`KismetMathLibrary.FClamp` (+ (.y (`self.K2_GetActorLocation` (`GameplayStatics.GetPlayerPawn` 0))) (`self.OffsetY`)) (`self.MinY`) (`self.MaxY`)) (`KismetMathLibrary.FClamp` (+ (.z (`self.K2_GetActorLocation` (`GameplayStatics.GetPlayerPawn` 0))) (`self.OffsetZ`)) (`self.MinZ`) (`self.MaxZ`))) DeltaTime (`self.FollowSpeed`))))

(fn `ViewUnbound`
  (params (DeltaTime :type "Float (single-precision)"))
  (`self.K2_SetActorLocation` (`KismetMathLibrary.VInterpTo` (`self.K2_GetActorLocation`) (`KismetMathLibrary.MakeVector` (+ (`self.OffsetX`) (.x (`self.K2_GetActorLocation` (`GameplayStatics.GetPlayerPawn` 0)))) (`self.LockedY`) (+ (.z (`self.K2_GetActorLocation` (`GameplayStatics.GetPlayerPawn` 0))) (`self.OffsetZ`))) DeltaTime (`self.FollowSpeed`))))

(fn `ViewUnboundUnlockedY`
  (params (DeltaTime :type "Float (single-precision)"))
  (`self.K2_SetActorLocation` (`KismetMathLibrary.VInterpTo` (`self.K2_GetActorLocation`) (`KismetMathLibrary.MakeVector` (+ (`self.OffsetX`) (.x (`self.K2_GetActorLocation` (`GameplayStatics.GetPlayerPawn` 0)))) (+ (.y (`self.K2_GetActorLocation` (`GameplayStatics.GetPlayerPawn` 0))) (`self.OffsetY`)) (+ (.z (`self.K2_GetActorLocation` (`GameplayStatics.GetPlayerPawn` 0))) (`self.OffsetZ`))) DeltaTime (`self.FollowSpeed`))))