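; AI controller for BP_TopDownEnemyAI that runs BT_EnemyAI and turns perception of the player into chase state.
; Sensing a living player sets hasSeenPlayer, ChaseTarget and the pawn's IsChasing flag.
; A dead player clears these and records LastKnownLocation, as does losing the player after a retriggerable delay that re-sensing does not cancel.
; ForgetPlayer clears only the target and seen blackboard keys.
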(event `self.ReceiveBeginPlay`
  (`self.RunBehaviorTree` "/Game/AI/BT_EnemyAI.BT_EnemyAI")
  (bind _asbp_top_down_enemy_ai (cast `/Game/Blueprints/Characters/Enemies/BP_TopDownEnemyAI` (`self.K2_GetPawn`)))
  (set `self.EnemyRef` _asbp_top_down_enemy_ai))

(event `self.AIPerception.OnTargetPerceptionUpdated`
  (params (Actor :type "Actor Object Reference") (Stimulus :type "AIStimulus Structure"))
  (bind (_age _expirationage _strength _stimuluslocation _receiverlocation _tag _bsuccessfullysensed) (break `AIStimulus` Stimulus))
  (bind _returnvalue (`AIBlueprintHelperLibrary.GetBlackboard` null))
  (bind _enemyref (`self.EnemyRef`))
  (bind _asbp_top_down_char (cast `/Game/Blueprints/Characters/Players/BP_TopDownChar` Actor))
  (if _bsuccessfullysensed
    (if (`/Game/Blueprints/Characters/Players/BP_TopDownChar.isDead` _asbp_top_down_char)
      (`BlackboardComponent.SetValueAsBool` _returnvalue "hasSeenPlayer" false :!label _label)
      (set `/Game/Blueprints/Characters/Enemies/BP_TopDownEnemyAI.isChasing` false _enemyref)
      (`BlackboardComponent.SetValueAsObject` _returnvalue "ChaseTarget" null)
      (`BlackboardComponent.SetValueAsVector` _returnvalue "LastKnownLocation" _stimuluslocation)
      (else
        (`BlackboardComponent.SetValueAsBool` _returnvalue "hasSeenPlayer" true)
        (set `/Game/Blueprints/Characters/Enemies/BP_TopDownEnemyAI.isChasing` true _enemyref)
        (`BlackboardComponent.SetValueAsObject` _returnvalue "ChaseTarget" _asbp_top_down_char)))
    (else
      (`KismetSystemLibrary.RetriggerableDelay` 3.0)
      (goto _label))))

(event `ForgetPlayer`
  (bind _returnvalue (`AIBlueprintHelperLibrary.GetBlackboard` null))
  (`BlackboardComponent.SetValueAsObject` _returnvalue "ChaseTarget" null)
  (`BlackboardComponent.SetValueAsBool` _returnvalue "hasSeenPlayer" false))

(fn `UserConstructionScript`)